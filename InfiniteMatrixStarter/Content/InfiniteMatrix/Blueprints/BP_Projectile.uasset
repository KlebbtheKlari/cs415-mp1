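; Projectile actor that flies along the world X axis in the Infinite Matrix game.
; Each tick it moves with a swept offset at a multiple of the Player's forward speed, scaled by delta time.
; Its Sphere component destroys the projectile when it begins overlapping a HealthPack or stops overlapping a BP_Tunnel.
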(event `self.ReceiveTick`
  (params (DeltaSeconds :type "Float (single-precision)"))
  (`self.K2_AddActorWorldOffset` (`KismetMathLibrary.MakeVector` (* DeltaSeconds (* (`/Game/InfiniteMatrix/Blueprints/BP_Player.ForwardSpeed` (`self.Player`)) 5.0))) true))

(event `self.Sphere.OnComponentBeginOverlap`
  (params (OverlappedComponent :type "PrimitiveComponent Object Reference") (OtherActor :type "Actor Object Reference") (OtherComp :type "PrimitiveComponent Object Reference") (OtherBodyIndex :type Integer) (bFromSweep :type Boolean) (SweepResult :type "HitResult Structure (by ref)"))
  (cast `/Game/InfiniteMatrix/Blueprints/HealthPack` OtherActor)
  (`self.K2_DestroyActor`))

(event `self.Sphere.OnComponentEndOverlap`
  (params (OverlappedComponent :type "PrimitiveComponent Object Reference") (OtherActor :type "Actor Object Reference") (OtherComp :type "PrimitiveComponent Object Reference") (OtherBodyIndex :type Integer))
  (cast `/Game/InfiniteMatrix/Blueprints/BP_Tunnel` OtherActor)
  (`self.K2_DestroyActor`))

(fn `UserConstructionScript`)